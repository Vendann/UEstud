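; BP_Svetofor is a traffic light that cycles endlessly through red, yellow, green and yellow, starting at red on BeginPlay.
; Red, Yellow and Green events swap materials on three lamp components to switch between color variants, then hand off after fixed delays.
; A FlipFlop in the shared Yellow event alternates the next phase between Green and Red, so one event serves both transitions.
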(event `self.ReceiveBeginPlay`
  (`self.Red`))

(event `Red`
  (`PrimitiveComponent.SetMaterial` (`self.LampX_1`) 0 "/Game/UE5/Svetofor/Materials/MI_Red.MI_Red")
  (`PrimitiveComponent.SetMaterial` (`self.LampX_2`) 0 "/Game/UE5/Svetofor/Materials/MI_Yellow1.MI_Yellow1")
  (`KismetSystemLibrary.Delay` 3.0)
  (`self.Yellow`))

(event `Yellow`
  (`PrimitiveComponent.SetMaterial` (`self.LampX_1`) 0 "/Game/UE5/Svetofor/Materials/MI_Red1.MI_Red1")
  (`PrimitiveComponent.SetMaterial` (`self.LampX_2`) 0 "/Game/UE5/Svetofor/Materials/MI_Yellow.MI_Yellow")
  (`PrimitiveComponent.SetMaterial` (`self.LampX_3`) 0 "/Game/UE5/Svetofor/Materials/MI_Green1.MI_Green1")
  (`KismetSystemLibrary.Delay` 1.0)
  (`/Engine/EditorBlueprintResources/StandardMacros.FlipFlop`
    (:`A`
      (`self.Green`))
    (:`B`
      (`self.Red`))))

(event `Green`
  (`PrimitiveComponent.SetMaterial` (`self.LampX_2`) 0 "/Game/UE5/Svetofor/Materials/MI_Yellow1.MI_Yellow1")
  (`PrimitiveComponent.SetMaterial` (`self.LampX_3`) 0 "/Game/UE5/Svetofor/Materials/MI_Green.MI_Green")
  (`KismetSystemLibrary.Delay` 3.0)
  (`self.Yellow`))

(event `CustomEvent`)

(fn `UserConstructionScript`)