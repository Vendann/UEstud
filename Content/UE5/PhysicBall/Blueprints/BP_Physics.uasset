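; BP_Physics is a physics-driven ball that moves in a random planar direction and rebounds off BP_Cube actors.
; On BeginPlay it picks a random normalized X/Y direction and scales it into a stored force vector.
; Each Tick applies that force to the Sphere as a mass-independent acceleration.
; Hitting a BP_Cube reflects the stored force about the hit normal, while other hits leave it unchanged.
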(event `self.ReceiveBeginPlay`
  (set `self.Force` (* (`KismetMathLibrary.Normal` (`KismetMathLibrary.MakeVector` (`KismetMathLibrary.RandomFloatInRange` -1.0 1.0) (`KismetMathLibrary.RandomFloatInRange` -1.0 1.0))) 300.0)))

(event `self.ReceiveTick`
  (params (DeltaSeconds :type "Float (single-precision)"))
  (`PrimitiveComponent.AddForce` (`self.Sphere`) (`self.Force`) "None" true))

(event `self.ReceiveHit`
  (params (MyComp :type "PrimitiveComponent Object Reference") (Other :type "Actor Object Reference") (OtherComp :type "PrimitiveComponent Object Reference") (bSelfMoved :type Boolean) (HitLocation :type "Vector Structure") (HitNormal :type "Vector Structure") (NormalImpulse :type "Vector Structure") (Hit :type "HitResult Structure (by ref)"))
  (cast `/Game/UE5/PhysicBall/Blueprints/BP_Cube` Other)
  (set `self.Force` (`KismetMathLibrary.GetReflectionVector` (`self.Force`) HitNormal)))

(fn `UserConstructionScript`)